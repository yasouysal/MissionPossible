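; Interactable fuse box that disables every security Camera in the level when used.
; BeginPlay binds to the Interactable's OnInteract delegate, which loops over all Camera actors with a valid blackboard.
; Each clears its isAlerted key, stops any Camera_Controller alarm sound and detaches from its controller, ending AI control.
; The switch sound plays at the box inside that loop, once per camera.
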(event `self.ReceiveBeginPlay`
  (add `Interactable.OnInteractDelegate` (`self.Interactable`) (delegate `OnInteract`)))

(event `OnInteract`
  (bind _outactors (`GameplayStatics.GetAllActorsOfClass` "/Game/AI/AI_Camera/Camera.Camera_C"))
  (for _array_element _outactors
    (bind _returnvalue (`AIBlueprintHelperLibrary.GetBlackboard` _array_element))
    (if (`KismetSystemLibrary.IsValid` _returnvalue)
      (`BlackboardComponent.SetValueAsBool` _returnvalue "isAlerted" false)
      (`GameplayStatics.PlaySoundAtLocation` "/Game/Sounds/79237__joedeshon__electrical_switch_01.79237__joedeshon__electrical_switch_01" (`self.K2_GetActorLocation`) (struct) 1.0 1.0 0.0 null null null null)
      (bind _ascamera_controller (cast `/Game/AI/AI_Camera/Camera_Controller` (`AIBlueprintHelperLibrary.GetAIController` _array_element))
        (:`then`
          (bind _alarmsound (`/Game/AI/AI_Camera/Camera_Controller.AlarmSound` _ascamera_controller))
          (if (`KismetSystemLibrary.IsValid` _alarmsound)
            (`AudioComponent.Stop` _alarmsound)))
        (:`CastFailed`
          _))
      (`Pawn.DetachFromControllerPendingDestroy` _array_element))))

(fn `UserConstructionScript`)
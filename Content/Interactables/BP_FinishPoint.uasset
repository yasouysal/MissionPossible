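; BP_FinishPoint is an interactable mission exit that ends the game when the player meets its completion condition.
; It binds to its Interactable's interact delegate on BeginPlay.
; On interaction, a never-detected player finishes immediately, while an ever-detected player must have every Enemy_Character dead, checked through each HealthManager.
; Success broadcasts game finished through BP_MissionPossibleGameState; otherwise nothing happens.
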(event `self.ReceiveBeginPlay`
  (add `Interactable.OnInteractDelegate` (`self.Interactable`) (delegate `OnInteract`)))

(event `OnInteract`
  (set `self.isAnyAIAlive` false)
  (bind _asbp_third_person_character (cast `/Game/ThirdPerson/Blueprints/BP_ThirdPersonCharacter` (`GameplayStatics.GetPlayerPawn` 0)))
  (if (`/Game/ThirdPerson/Blueprints/BP_ThirdPersonCharacter.isEverDetected` _asbp_third_person_character)
    (bind _outactors (`GameplayStatics.GetAllActorsOfClass` "/Game/AI/AI_Character/Enemy_Character.Enemy_Character_C"))
    (for _array_element _outactors
      (bind _returnvalue (`HealthManager.CheckisDead` (`/Game/AI/AI_Character/Enemy_Character.HealthManager` _array_element)))
      (if (not _returnvalue)
        (set `self.isAnyAIAlive` true)))
    (if (not (`self.isAnyAIAlive`))
      (bind _asbp_mission_possible_game_state (cast `/Game/GameModeBPs/BP_MissionPossibleGameState` (`GameplayStatics.GetGameState`)))
      (`/Game/GameModeBPs/BP_MissionPossibleGameState.BroadcastGameFinished` _asbp_mission_possible_game_state))
    (else
      (bind _asbp_mission_possible_game_state_2 (cast `/Game/GameModeBPs/BP_MissionPossibleGameState` (`GameplayStatics.GetGameState`)))
      (`/Game/GameModeBPs/BP_MissionPossibleGameState.BroadcastGameFinished` _asbp_mission_possible_game_state_2))))

(fn `UserConstructionScript`)